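; Controller detection utility that spots changes of input device and handles main menu opening, closing and rebuilding.
; HasControllerChanged sorts the last key into two gamepad types, by whether its display name contains "Gamepad", or non-gamepad, then compares it with the current controller.
; Menu helpers create Main_Menu for a controller type, or close widgets and trigger FP_Controller's ChangeMainMenuEvent, optionally passing the new controller and selected option.
; HideFromCursor makes a widget's children non-hit-testable.
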(fn `AreControllersDifferent`
  (params (currentController :type "/Game/Blueprints/Movement/ControlTypeEnum Enum" :default "NewEnumerator0") (newController :type "/Game/Blueprints/Movement/ControlTypeEnum Enum" :default "NewEnumerator0"))
  (returns (ReturnValue :type Boolean))
  (return (`|EnumInequality` currentController newController)))

(fn `CloseMenu`
  (params (currentWidget :type "UserWidget Object Reference"))
  (bind _returnvalue (`GameplayStatics.GetPlayerController` null))
  (`Widget.RemoveFromParent` currentWidget)
  (`WidgetBlueprintLibrary.SetInputMode_GameOnly` _returnvalue)
  (set `PlayerController.bShowMouseCursor` false _returnvalue)
  (return))

(fn `CloseToMain`
  (params (currentWidget :type "UserWidget Object Reference"))
  (`self.CloseMenu` currentWidget)
  (bind _returnvalue (`GameplayStatics.GetActorOfClass` null "/Game/Blueprints/Movement/FP_Controller.FP_Controller_C"))
  (`/Game/Blueprints/Movement/FP_Controller.ChangeMainMenu_Event` _returnvalue))

(fn `HasControllerChanged`
  (params (lastkey :type "Key Structure" :default "None") (currentController :type "/Game/Blueprints/Movement/ControlTypeEnum Enum" :default "NewEnumerator0"))
  (returns (hasChanged :type Boolean) (new :type "/Game/Blueprints/Movement/ControlTypeEnum Enum"))
  (if (`KismetInputLibrary.Key_IsGamepadKey` lastkey)
    (if (`KismetStringLibrary.Contains` (`KismetTextLibrary.Conv_TextToString` (`KismetInputLibrary.Key_GetDisplayName` lastkey)) "Gamepad")
      (if (`self.AreControllersDifferent` currentController)
        (return true "NewEnumerator0")
        (else
          _))
      (elif (`self.AreControllersDifferent` currentController "NewEnumerator1")
        (return true "NewEnumerator1")
        (else
          _)))
    (elif (`self.AreControllersDifferent` currentController "NewEnumerator2")
      (return true "NewEnumerator2")
      (else
        _)))
  (return false "NewEnumerator0"))

(fn `HideFromCursor`
  (params (FatherElement :type "CanvasPanel Object Reference"))
  (for _array_element (`PanelWidget.GetAllChildren` FatherElement)
    (`Widget.SetVisibility` _array_element "HitTestInvisible"))
  (return))

(fn `OpenMainMenu`
  (params (controller :type "/Game/Blueprints/Movement/ControlTypeEnum Enum" :default "NewEnumerator0"))
  (bind _returnvalue (`|CreateWidget` "/Game/Blueprints/Menus/Main_Menu.Main_Menu_C" null controller))
  (`WidgetBlueprintLibrary.SetInputMode_GameAndUIEx` (`GameplayStatics.GetPlayerController` null) _returnvalue "DoNotLock" false)
  (`UserWidget.AddToViewport` _returnvalue 0) ; POSIBLEMENTE CAMBIAR ESO
)

(fn `RemakeMainMenu`
  (params (newController :type "/Game/Blueprints/Movement/ControlTypeEnum Enum" :default "NewEnumerator0") (currentWidget :type "UserWidget Object Reference") (selectedOption :type Integer))
  (`self.CloseMenu` currentWidget)
  (bind _returnvalue (`GameplayStatics.GetActorOfClass` null "/Game/Blueprints/Movement/FP_Controller.FP_Controller_C"))
  (set `/Game/Blueprints/Movement/FP_Controller.LastControllerUsed` newController _returnvalue)
  (set `/Game/Blueprints/Movement/FP_Controller.SelectedOption` selectedOption _returnvalue)
  (`/Game/Blueprints/Movement/FP_Controller.ChangeMainMenu_Event` _returnvalue))