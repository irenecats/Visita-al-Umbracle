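; ButtonOverride is a menu button Blueprint that keeps its visual style in sync with mouse hover and keyboard focus.
; InitButton starts a fast looping timer that polls CheckFocus, rather than reacting to hover or focus events.
; CheckFocus gives a hovered button keyboard focus and the hover style, otherwise applying the selected or unselected style based on whether it holds focus.
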(fn `CheckFocus`
  (if (`self.IsHovered`)
    (`self.SetKeyboardFocus`)
    (`self.SetStyle` (`self.MouseHover`))
    (else
      (`self.SetStyle` (select `bool` (`self.HasKeyboardFocus`) :`false` (`self.NotSelected`) :`true` (`self.Selected`))))))

(fn `InitButton`
  (`KismetSystemLibrary.K2_SetTimer` self "CheckFocus" 0.01 true))