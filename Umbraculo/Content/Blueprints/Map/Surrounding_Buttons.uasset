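; Surrounding_Buttons holds a map button's neighbour references (Top, Down, Left, Right) alongside a Centre reference, apparently for directional navigation between buttons.
; Four getter functions each return the neighbour in that direction if it is valid, and otherwise fall back to Centre, so a missing neighbour resolves to the centre button.
; The event graph has no active logic.
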(fn `getDownButton`
  (returns (NewParam :type "/Game/Blueprints/Menus/ButtonOverride Object Reference"))
  (`/Engine/EditorBlueprintResources/StandardMacros.IsValid` (`self.Down`)
    (:`Is Valid`
      (return (`self.Down`)))
    (:`Is Not Valid`
      (return (`self.Centre`)))))

(fn `getLeftButton`
  (returns (NewParam :type "/Game/Blueprints/Menus/ButtonOverride Object Reference"))
  (`/Engine/EditorBlueprintResources/StandardMacros.IsValid` (`self.Left`)
    (:`Is Valid`
      (return (`self.Left`)))
    (:`Is Not Valid`
      (return (`self.Centre`)))))

(fn `getRightButton`
  (returns (NewParam :type "/Game/Blueprints/Menus/ButtonOverride Object Reference"))
  (`/Engine/EditorBlueprintResources/StandardMacros.IsValid` (`self.Right`)
    (:`Is Valid`
      (return (`self.Right`)))
    (:`Is Not Valid`
      (return (`self.Centre`)))))

(fn `getTopButton`
  (returns (NewParam :type "/Game/Blueprints/Menus/ButtonOverride Object Reference"))
  (`/Engine/EditorBlueprintResources/StandardMacros.IsValid` (`self.Top`)
    (:`Is Valid`
      (return (`self.Top`)))
    (:`Is Not Valid`
      (return (`self.Centre`)))))