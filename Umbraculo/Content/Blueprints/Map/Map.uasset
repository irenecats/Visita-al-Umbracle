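; Map Blueprint that drives the menu's map overlay, showing player and teleport icons with zoom support.
; TopLeft and BottomRight markers define the world bounds used to convert actor locations into widget translations.
; Player position and rotation are set when the map is prepared, not every tick.
; Zooming scales the map within clamped limits, optionally resizes icons, repositions them, and pulls the map toward center when zooming out.
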(event `ZoomMap`
  (params (ZoomAxis :type "Float (double-precision)") (ZoomAmount :type "Float (double-precision)"))
  (set `self.Axis` ZoomAxis)
  (`self.ModifyZoom` (+ 1.0 (* (`self.Axis`) (/ ZoomAmount 100.0)))))

(event `prepare Map`
  (params (`Map Menu` :type "/Game/Blueprints/Map/Map_menu Object Reference"))
  (bind _output_get (set `self.Map Main Menu` `Map Menu`))
  (bind _output_get_2 (set `self.Map Reference` (`/Game/Blueprints/Map/Map_menu.Map_overlay` _output_get)))
  (`/Game/Blueprints/Map/Map_overlay.Initialize` _output_get_2 self)
  (set `self.OriginalPlayerSize` (`/Game/Blueprints/Map/Map_overlay.PlayerSize` (`self.Map Reference`)))
  (set `self.OriginalMapSize` (`/Game/Blueprints/Map/Map_overlay.MapSize` (`self.Map Reference`)))
  (set `self.OriginalTeleportSize` (`/Game/Blueprints/Map/Map_overlay.TeleportSize` (`self.Map Reference`)))
  (`self.UpdatePlayerPosition`) ; Si quiero que se actualice mientras se muestra tendría que hacer un evento diferente
  (`self.UpdatePlayerRotation`))

(event `Init`
  (params (Player :type "Character Object Reference"))
  (`/Engine/EditorBlueprintResources/StandardMacros.IsValid` Player
    (:`Is Valid`
      (set `self.PlayerReference` Player))))

(fn `CenterMap`
  (if (< (`self.Axis`) 0.0)
    (`Widget.SetRenderTranslation` (`self.Map Reference`) (`KismetMathLibrary.Conv_VectorToVector2D` (`KismetMathLibrary.VLerp` (0.0 0.0 0.0) (`KismetMathLibrary.Conv_Vector2DToVector` (`.Translation` (break `WidgetTransform` (`Widget.RenderTransform` (`self.Map Reference`))))) (/ (`self.SizeMultiplier`) 8.0))))))

(fn `isMapOutOfBounds`
  (returns (`Out of Bounds` :type Boolean))
  (bind (_returnvalue_x _returnvalue_y) (`KismetMathLibrary.BreakVector2D` (`WidgetLayoutLibrary.GetViewportSize`)))
  (bind (_returnvalue_x_2 _returnvalue_y_2) (`KismetMathLibrary.BreakVector2D` (`Widget.GetDesiredSize` (`self.Map Reference`))))
  (return (or (> _returnvalue_x_2 _returnvalue_x) (> _returnvalue_y_2 _returnvalue_y))))

(fn `MapHeight`
  (returns (height :type "Float (double-precision)"))
  (bind (_returnvalue_x _returnvalue_y) (`KismetMathLibrary.BreakVector` (`Actor.K2_GetActorLocation` (`self.TopLeft`))))
  (bind (_returnvalue_x_2 _returnvalue_y_2) (`KismetMathLibrary.BreakVector` (`Actor.K2_GetActorLocation` (`self.BottomRight`))))
  (return (`KismetMathLibrary.Abs` (- _returnvalue_y _returnvalue_y_2))))

(fn `MapWidth`
  (returns (width :type "Float (double-precision)"))
  (bind _returnvalue_x (`KismetMathLibrary.BreakVector` (`Actor.K2_GetActorLocation` (`self.TopLeft`))))
  (bind _returnvalue_x_2 (`KismetMathLibrary.BreakVector` (`Actor.K2_GetActorLocation` (`self.BottomRight`))))
  (return (`KismetMathLibrary.Abs` (- _returnvalue_x _returnvalue_x_2))))

(fn `ModifyZoom`
  (params (Multiplier :type "Float (double-precision)"))
  (bind _map_reference (`self.Map Reference`))
  (if (> Multiplier 0.0)
    (set `self.SizeMultiplier` (`KismetMathLibrary.FClamp` (* Multiplier (`self.SizeMultiplier`)) 0.8 7.0))
    (`/Game/Blueprints/Map/Map_overlay.setMapSize` (`self.Map Reference`) (`KismetMathLibrary.ToRounded2D` (* (`self.OriginalMapSize`) (`self.SizeMultiplier`))))
    (if (`self.ChangeIconsSize`)
      (`/Game/Blueprints/Map/Map_overlay.setPlayerSize` _map_reference (`KismetMathLibrary.ToRounded2D` (* (`self.OriginalPlayerSize`) (`self.SizeMultiplier`))))
      (`/Game/Blueprints/Map/Map_overlay.setTeleportsSize` _map_reference (`KismetMathLibrary.ToRounded2D` (* (`self.OriginalTeleportSize`) (`self.SizeMultiplier`)))))
    (`self.UpdatePlayerPosition`)
    (`self.UpdateTpPosition`)
    (`self.CenterMap`)
    (return)
    (else
      (return))))

(fn `UpdatePlayerPosition`
  (bind _widgetposition (`self.WorldToWidgetLocation` (`Actor.K2_GetActorLocation` (`self.PlayerReference`)) (`self.OriginalPlayerSize`)))
  (`Widget.SetRenderTranslation` (`/Game/Blueprints/Map/Map_overlay.Player` (`self.Map Reference`)) _widgetposition)
  (return))

(fn `UpdatePlayerRotation`
  (bind (_returnvalue_roll _returnvalue_pitch _returnvalue_yaw) (`KismetMathLibrary.BreakRotator` (`Actor.K2_GetActorRotation` (`self.PlayerReference`))))
  (`Widget.SetRenderTransformAngle` (`/Game/Blueprints/Map/Map_overlay.Player` (`self.Map Reference`)) (+ _returnvalue_yaw 90.0))
  (return))

(fn `UpdateTpPosition`
  (for _array_element (`PanelWidget.GetAllChildren` (`/Game/Blueprints/Map/Map_overlay.Teleports_overlay` (`self.Map Reference`)))
    (bind _asmap_tp_icon (cast `/Game/Blueprints/Map/Map_TP_icon` _array_element))
    (bind _widgetposition (`self.WorldToWidgetLocation` (`Actor.K2_GetActorLocation` (`/Game/Blueprints/Map/Map_TP_icon.Teleport Reference` _asmap_tp_icon)) (`self.OriginalTeleportSize`)))
    (`Widget.SetRenderTranslation` _array_element _widgetposition)))

(fn `WorldToMapLocation`
  (params (WorldLocation :type "Vector Structure"))
  (returns (MapLocation :type "Vector2D Structure"))
  (bind (_returnvalue_x _returnvalue_y) (`KismetMathLibrary.BreakVector` (`KismetMathLibrary.Vector_GetAbs` (- WorldLocation (`Actor.K2_GetActorLocation` (`self.TopLeft`))))))
  (return (`KismetMathLibrary.MakeVector2D` _returnvalue_x _returnvalue_y)))

(fn `WorldToWidgetLocation`
  (params (Location :type "Vector Structure") (WidgetSize :type "Vector2D Structure"))
  (returns (WidgetPosition :type "Vector2D Structure"))
  (bind (_maplocation_x _maplocation_y) (`KismetMathLibrary.BreakVector2D` (`self.WorldToMapLocation` Location)))
  (bind (_returnvalue_x _returnvalue_y) (`KismetMathLibrary.BreakVector2D` (/ WidgetSize 2.0)))
  (bind (_mapsize_x _mapsize_y) (`KismetMathLibrary.BreakVector2D` (`/Game/Blueprints/Map/Map_overlay.MapSize` (`self.Map Reference`))))
  (return (`KismetMathLibrary.MakeVector2D` (- (* (/ _maplocation_x (`self.MapWidth`)) _mapsize_x) _returnvalue_x) (- (* _mapsize_y (/ _maplocation_y (`self.MapHeight`))) _returnvalue_y))))